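; Base rifle actor that fires projectiles on behalf of the Pawn it is attached to as a child actor.
; On BeginPlay it caches its parent Pawn, or prints a debug string and destroys itself if there is none.
; Attack spawns the projectile at the muzzle socket along the Pawn's base aim rotation, with the Pawn as instigator and its controller as owner.
; A busy flag and reset timer limit the fire rate.
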(event `self.ReceiveBeginPlay`
  (`parent.ReceiveBeginPlay`)
  (bind _aspawn (cast `Pawn` (`self.GetParentActor`))
    (:`then`
      (set `self.ParentPawn` _aspawn))
    (:`CastFailed`
      (`KismetSystemLibrary.PrintString` "Hello")
      (`self.K2_DestroyActor`))))

(event `ActionStopped`
  (set `self.ActionHappening` false))

(fn `Attack`
  (bind _parentpawn (`self.ParentPawn`))
  (if (`self.CanShoot`)
    (`|SpawnActorFromClass` (`self.ProjectileClass`) (`KismetMathLibrary.MakeTransform` (`SceneComponent.GetSocketLocation` (`self.SK_Rifle`) (`self.MuzzleFlashSocket`)) (`Pawn.GetBaseAimRotation` (`self.ParentPawn`))) "Undefined" "MultiplyWithRoot" (`Pawn.GetController` _parentpawn) _parentpawn)
    (set `self.ActionHappening` true)
    (`KismetSystemLibrary.K2_SetTimerDelegate` (`|CreateDelegate` :!event `ActionStopped`) (`self.ResetTime`))))

(fn `CanShoot`
  (returns (Yes :type Boolean))
  (return (not (`self.ActionHappening`))))

(fn `UserConstructionScript`)